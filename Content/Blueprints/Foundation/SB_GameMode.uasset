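; SB_GameMode is a game mode Blueprint that hosts the planning UI and keeps the list of waypoints.
; On BeginPlay it creates the UMG_Planning widget if no valid reference exists and adds it to the viewport.
; AddWaypoint appends a waypoint to the list and passes its location and new index to the paths manager, when that reference is valid, to add a marker.
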(event EventBeginPlay
  (CallFunction|UMGInitialize))

(event EventTick
  (params (DeltaSeconds :type Float%20%28single-precision%29)))

(fn ConstructionScript)

(fn UMGInitialize
  (Variables|Default|GetPlanningUMGRef
    (:then
      _)
    (:else
      (bind _returnvalue (UserInterface|CreateWidget "/Game/UI/UMG_Planning.UMG_Planning_C"))
      (bind _output_get (Variables|Default|SetPlanningUMGRef _returnvalue))))
  (UserInterface|Viewport|AddtoViewport _output_get 0))

(fn AddWaypoint
  (params (Waypoint :type Struct%20Waypoint%20Structure%20%28by%20ref%29))
  (bind _returnvalue (Utilities|Array|Add (Variables|Default|GetWaypointsList) Waypoint))
  (LocalVariables|Set_Index _returnvalue)
  (Utilities|FlowControl|Sequence
    (:then_0
      (bind _pathsmanagerref (Variables|References|GetPathsManagerRef)
        (:then
          (Default|AddWaypointMarker _pathsmanagerref Waypoint (LocalVariables|Get_Index)))
        (:else)))))