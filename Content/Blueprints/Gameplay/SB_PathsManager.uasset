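; SB_PathsManager spawns waypoint markers and builds a navigation path through them as a spline, registering itself with SB_GameMode on BeginPlay.
; AddWaypointMarker spawns an attached marker facing the spectator camera's yaw, stores it by index, then calls UpdatePath.
; UpdatePath runs navmesh pathfinding between consecutive markers and adds unique points to a never-cleared array.
; That array becomes linear spline points, applied in local space.
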(event EventBeginPlay
  (bind _assb_spectator_pawn (Utilities|Casting|CastToSB_SpectatorPawn (Game|Player|GetPlayerPawn 0)))
  (Variables|References|SetSpectatorRef _assb_spectator_pawn)
  (bind _assb_game_mode (Utilities|Casting|CastToSB_GameMode (Game|GetGameMode)))
  (bind _output_get (Variables|References|SetGameModeRef _assb_game_mode))
  (Variables|/Game/Blueprints/Foundation/SB_GameMode.SB_GameMode_C|SetPathsManagerRef _output_get self))

(event EventTick
  (params (DeltaSeconds :type Float%20%28single-precision%29)))

(fn ConstructionScript
  (Spline|SetSplinePointType (Variables|Default|GetSpline) 0 "Linear" true))

(fn AddWaypointMarker
  (params (Location :type Struct%20Waypoint%20Structure%20%28by%20ref%29) (Index :type Integer))
  (LocalVariables|Set_Index Index)
  (LocalVariables|Set_Location (.Location (Utilities|Struct|BreakStruct_Waypoint Location)))
  (Utilities|FlowControl|Sequence
    (:then_0
      ;[1 1 1] Spawn waypoint marker
      (bind _returnvalue (Game|SpawnActorfromClass "/Game/Blueprints/Gameplay/SB_WaypointMarker.SB_WaypointMarker_C" (Math|Transform|MakeTransform (LocalVariables|Get_Location) (Math|Rotator|MakeRotator 0.0 0.0 (Variables|/Game/Blueprints/Player/SB_SpectatorPawn.SB_SpectatorPawn_C|GetCamYaw (Variables|References|GetSpectatorRef)))) "Undefined" 0 0))
      (bind _output_get (LocalVariables|Set_MarkerRef _returnvalue))
      (Transformation|AttachActorToActor _output_get self "None" "KeepWorld" "KeepWorld" "KeepWorld" true))
    (:then_1
      ;[1 1 1] Set values
      (Default|SetValues (LocalVariables|Get_MarkerRef) (LocalVariables|Get_Index))
      (Utilities|Map|Add (Variables|Default|GetSpawnedWPMarkers) (LocalVariables|Get_Index) (LocalVariables|Get_MarkerRef)))
    (:then_2
      (CallFunction|UpdatePath))))

(fn UpdatePath
  (Utilities|FlowControl|Sequence
    (:then_0
      ;[1 1 1] Get path points for all waypoints
      (for _index (range 1 (- (Utilities|Map|Length (Variables|Default|GetSpawnedWPMarkers)) 1))
        (bind _returnvalue (Class|NavigationSystem|FindPathtoActorSynchronously (Transformation|GetActorLocation (.Value (Utilities|Map|Find (Variables|Default|GetSpawnedWPMarkers) (- _index 1)))) (.Value (Utilities|Map|Find (Variables|Default|GetSpawnedWPMarkers) _index)) 5e+01))
        (for _array_element (Variables|/Script/Engine.NavigationPath|GetPathPoints _returnvalue)
          (Utilities|Array|AddUnique (LocalVariables|Get_SplinePoints) _array_element))))
    (:then_1
      ;[1 1 1] Set Spline
      (Spline|SetSplinePoints (Variables|Default|GetSpline) (LocalVariables|Get_SplinePoints) "Local" false)
      (for _index_2 (range 0 (- (Spline|GetNumberOfSplinePoints (Variables|Default|GetSpline)) 1))
        (Spline|SetSplinePointType (Variables|Default|GetSpline) _index_2 "Linear" false))
      (Spline|UpdateSpline (Variables|Default|GetSpline)))))