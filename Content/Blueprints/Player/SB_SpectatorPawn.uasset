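; Spectator pawn that drives an orthographic camera with axis-input panning, clamped zoom and optional mouse edge scrolling.
; Tick feeds screen-edge scrolling into the same move functions as the input axes, offsetting the pawn along camera-relative directions.
; The first overlapped BlockingVolume becomes the camera bounds.
; After leaving a volume, moves pointing away from the bounds' center are rejected, a soft limit without clamping position.
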(event EventBeginPlay)

(event Collision|EventActorBeginOverlap
  (params (OtherActor :type Actor%20Object%20Reference))
  (bind _asblocking_volume (Utilities|Casting|CastToBlockingVolume OtherActor))
  (Variables|Camera|GetCamBounds
    (:then
      _)
    (:else
      (Variables|Camera|SetCamBounds _asblocking_volume)))
  (Variables|Camera|SetCamOutOfBounds false))

(event Collision|EventActorEndOverlap
  (params (OtherActor :type Actor%20Object%20Reference))
  (Utilities|Casting|CastToBlockingVolume OtherActor)
  (Variables|Camera|SetCamOutOfBounds true))

(event EventTick
  (params (DeltaSeconds :type Float%20%28single-precision%29))
  (CallFunction|Scrolling DeltaSeconds))

(event Input|AxisEvents|InputAxisZoom
  (params (AxisValue :type Float%20%28single-precision%29))
  (if (Variables|Camera|GetCamCanMove)
    (Class|CameraComponent|SetOrthoWidth (Variables|Default|GetCamera) (Math|Float|Clamp(Float) (+ (* AxisValue (Variables|Camera|GetCamZoomSpeed)) (Variables|/Script/Engine.CameraComponent|GetOrthoWidth (Variables|Default|GetCamera))) (Variables|Camera|GetCamZoomMin) (Variables|Camera|GetCamZoomMax)))))

(event Input|AxisEvents|InputAxisMoveForward
  (params (AxisValue :type Float%20%28single-precision%29))
  (if (Variables|Camera|GetCamCanMove)
    (CallFunction|MoveCamForward AxisValue)))

(event Input|AxisEvents|InputAxisMoveRight
  (params (AxisValue :type Float%20%28single-precision%29))
  (if (Variables|Camera|GetCamCanMove)
    (CallFunction|MoveCamRight AxisValue)))

(fn ConstructionScript)

(fn Scrolling
  (params (DeltaSeconds :type Float%20%28single-precision%29))
  (bind _camscrollboundary (Variables|Camera|GetCamScrollBoundary))
  (bind _camscrollboundary_2 (Variables|Camera|GetCamScrollBoundary))
  (if (Variables|Camera|GetCamScrollingEnabled)
    (LocalVariables|Set_Delta (* DeltaSeconds 1e+01 (Variables|Camera|GetCamMoveSpeed)))
    (if (Variables|Camera|GetCamCanMove)
      (Utilities|FlowControl|Sequence
        (:then_0
          (bind _returnvalue (Class|WidgetLayoutLibrary|GetMousePositiononViewport))
          (LocalVariables|Set_MousePos _returnvalue)
          (LocalVariables|Set_ViewportSize (Viewport|GetViewportSize)))
        (:then_1
          (if (< (.x (LocalVariables|Get_MousePos)) _camscrollboundary_2)
            (CallFunction|MoveCamRight (* (LocalVariables|Get_Delta) -1.0))
            (elif (< (- (.x (LocalVariables|Get_ViewportSize)) (.x (LocalVariables|Get_MousePos))) _camscrollboundary_2)
              (CallFunction|MoveCamRight (LocalVariables|Get_Delta)))))
        (:then_2
          (if (< (.y (LocalVariables|Get_MousePos)) _camscrollboundary)
            (CallFunction|MoveCamForward (LocalVariables|Get_Delta))
            (elif (< (- (.y (LocalVariables|Get_ViewportSize)) (.y (LocalVariables|Get_MousePos))) _camscrollboundary)
              (CallFunction|MoveCamForward (* (LocalVariables|Get_Delta) -1.0)))))))))

(fn MoveCamForward
  (params (AxisValue :type Float%20%28single-precision%29))
  (LocalVariables|Set_DeltaLocation (* (Math|Vector|GetForwardVector (Utilities|GetIsolatedCameraYaw)) (* AxisValue (Variables|Camera|GetCamMoveSpeed))))
  (Utilities|FlowControl|Sequence
    (:then_0
      (if (Variables|Camera|GetCamOutOfBounds)
        (bind _cambounds (Variables|Camera|GetCamBounds)
          (:then
            (if (not (>= (Math|Vector|DotProduct (Math|Vector|Normalize (LocalVariables|Get_DeltaLocation)) (Math|Vector|Normalize (- (.Origin (Collision|GetActorBounds _cambounds false)) (Transformation|GetActorLocation)))) 0.0))
              (return)))
          (:else))))
    (:then_1
      (Transformation|AddActorLocalOffset self (LocalVariables|Get_DeltaLocation) false false))))

(fn MoveCamRight
  (params (AxisValue :type Float%20%28single-precision%29))
  (LocalVariables|Set_DeltaLocation (* (Math|Vector|GetRightVector (Utilities|GetIsolatedCameraYaw)) (* AxisValue (Variables|Camera|GetCamMoveSpeed))))
  (Utilities|FlowControl|Sequence
    (:then_0
      (if (Variables|Camera|GetCamOutOfBounds)
        (bind _cambounds (Variables|Camera|GetCamBounds)
          (:then
            (if (not (>= (Math|Vector|DotProduct (Math|Vector|Normalize (LocalVariables|Get_DeltaLocation)) (Math|Vector|Normalize (- (.Origin (Collision|GetActorBounds _cambounds false)) (Transformation|GetActorLocation)))) 0.0))
              (return)))
          (:else))))
    (:then_1
      (Transformation|AddActorLocalOffset self (LocalVariables|Get_DeltaLocation) false false))))